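; BP_SpeedBoost is a status effect that changes the movement speed of the player it references.
; When the effect turns on, it multiplies the CharacterMovement MaxWalkSpeed by the intensity value from StatusInfo.
; When it turns off, it divides by that same value to undo the change, without caching the original speed.
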(event `self.StatusEffectOn`
  (bind (_statusinfo_statusname _statusinfo_statusicon _statusinfo_description _statusinfo_statustype _statusinfo_duration _statusinfo_intensityvalue) (break `/Game/Statuses/STR_StatusInfo` (`self.StatusInfo`)))
  (bind _charactermovement (`Character.CharacterMovement` (`self.PlayerReference`)))
  (set `CharacterMovementComponent.MaxWalkSpeed` (* (`CharacterMovementComponent.MaxWalkSpeed` _charactermovement) _statusinfo_intensityvalue) _charactermovement))

(event `self.StatusEffectOff`
  (bind (_statusinfo_statusname _statusinfo_statusicon _statusinfo_description _statusinfo_statustype _statusinfo_duration _statusinfo_intensityvalue) (break `/Game/Statuses/STR_StatusInfo` (`self.StatusInfo`)))
  (bind _charactermovement (`Character.CharacterMovement` (`self.PlayerReference`)))
  (set `CharacterMovementComponent.MaxWalkSpeed` (/ (`CharacterMovementComponent.MaxWalkSpeed` _charactermovement) _statusinfo_intensityvalue) _charactermovement))

(fn `UserConstructionScript`
  (`parent.UserConstructionScript`))