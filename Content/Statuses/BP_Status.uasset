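; BP_Status is the base actor for timed status effects applied to the player, with child classes overriding the on and off effect hooks.
; ApplyStatus registers the status on the player pawn, runs StatusEffectOn, adds it to the HUD status bar and starts a timer from StatusInfo's duration.
; When the timer fires, RemoveStatus runs StatusEffectOff, clears the bar and pawn entries, and destroys the actor.
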(event `self.ReceiveBeginPlay`
  (bind _asbp_player_pawn (cast `/Game/Player/BP_PlayerPawn` (`GameplayStatics.GetPlayerPawn` 0)))
  (set `self.PlayerReference` _asbp_player_pawn))

(event `ApplyStatus`
  (params (PlayerPawn :type "/Game/Player/BP_PlayerPawn Object Reference") (PlayerController :type "/Game/Core/BP_PlayerController Object Reference"))
  (bind (_statusinfo_statusname _statusinfo_statusicon _statusinfo_description _statusinfo_statustype _statusinfo_duration) (break `/Game/Statuses/STR_StatusInfo` (`self.StatusInfo`)))
  (bind _output_get (set `self.PlayerController` PlayerController))
  (set `self.StatusBar` (`/Game/UI/WBP_Main.WBP_StatusBar` (`/Game/Core/BP_PlayerController.HUDMain` _output_get)))
  (bind _output_get_2 (set `self.PlayerReference` PlayerPawn))
  (`KismetArrayLibrary.Array_Add` (`/Game/Player/BP_PlayerPawn.CurrentStatuses` _output_get_2) self)
  (`self.StatusEffectOn`)
  (`/Game/UI/WBP_StatusBar.AddStatusToBar` (`self.StatusBar`) self)
  (bind _returnvalue (`KismetSystemLibrary.K2_SetTimerDelegate` (delegate `RemoveStatus`) _statusinfo_duration)))

(event `StatusEffectOn`
  ;[1 0.275 0.275] Override in Child
)

(event `StatusEffectOff`
  ;[1 0.275 0.275] Override in Child
)

(event `RemoveStatus`
  (`self.StatusEffectOff`)
  (`/Game/UI/WBP_StatusBar.RemoveStatusFromBar` (`self.StatusBar`) self)
  (`KismetArrayLibrary.Array_RemoveItem` (`/Game/Player/BP_PlayerPawn.CurrentStatuses` (`self.PlayerReference`)) self)
  (`KismetSystemLibrary.K2_ClearAndInvalidateTimerHandle` (stale `ApplyStatus` _returnvalue))
  (`self.K2_DestroyActor`))

(fn `UserConstructionScript`)