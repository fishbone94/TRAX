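; BP_Immobilize is a status effect that stops the player from walking or crouch-walking while it is active.
; When switched on, it saves the player's CharacterMovement walk and crouched speed limits, then sets both to zero.
; When switched off, it restores the saved speeds.
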(event `self.StatusEffectOn`
  (bind _charactermovement (`Character.CharacterMovement` (`self.PlayerReference`)))
  (set `self.PrevMaxWalkSpeed` (`CharacterMovementComponent.MaxWalkSpeed` _charactermovement))
  (set `self.PrevMaxCrouchSpeed` (`CharacterMovementComponent.MaxWalkSpeedCrouched` _charactermovement))
  (set `CharacterMovementComponent.MaxWalkSpeed` 0.0 _charactermovement)
  (set `CharacterMovementComponent.MaxWalkSpeedCrouched` 0.0 _charactermovement))

(event `self.StatusEffectOff`
  (bind _charactermovement (`Character.CharacterMovement` (`self.PlayerReference`)))
  (set `CharacterMovementComponent.MaxWalkSpeed` (`self.PrevMaxWalkSpeed`) _charactermovement)
  (set `CharacterMovementComponent.MaxWalkSpeedCrouched` (`self.PrevMaxCrouchSpeed`) _charactermovement))

(fn `UserConstructionScript`
  (`parent.UserConstructionScript`))