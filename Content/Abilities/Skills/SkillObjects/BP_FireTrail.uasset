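; BP_FireTrail is a short-lived fire hazard skill object that burns players who enter it, unless their current element is Fire.
; It sets its own lifespan on BeginPlay and checks Box overlaps for player pawns and their controllers.
; For each valid overlap it spawns a BP_Burning status actor, fills its status info from the burn duration and intensity variables, and applies it to that player.
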(event `self.ReceiveBeginPlay`
  (`self.SetLifeSpan` 10.0))

(event `self.Box.OnComponentBeginOverlap`
  (params (OverlappedComponent :type "PrimitiveComponent Object Reference") (OtherActor :type "Actor Object Reference") (OtherComp :type "PrimitiveComponent Object Reference") (OtherBodyIndex :type Integer) (bFromSweep :type Boolean) (SweepResult :type "HitResult Structure (by ref)"))
  (if (`KismetMathLibrary.ClassIsChildOf` (`GameplayStatics.GetObjectClass` OtherActor) "/Game/Player/BP_PlayerPawn.BP_PlayerPawn_C")
    (bind _asbp_player_pawn (cast `/Game/Player/BP_PlayerPawn` OtherActor))
    (bind _asbp_player_controller (cast `/Game/Core/BP_PlayerController` (`Pawn.GetController` _asbp_player_pawn)))
    (if (not (== (`/Game/Core/BP_PlayerController.CurrentElement` _asbp_player_controller) "/Game/Abilities/Elements/BP_ElementFire.BP_ElementFire_C"))
      (bind _returnvalue (`|SpawnActorFromClass` "/Game/Statuses/BP_Burning.BP_Burning_C" (`self.GetTransform`) "Undefined" "OverrideRootScale"))
      (set `/Game/Statuses/BP_Status.StatusInfo` (make `/Game/Statuses/STR_StatusInfo` "Burning" "/Game/UI/Assets/T_Burning_Icon.T_Burning_Icon" "" "NewEnumerator2" (`self.BurnDuration`) (`self.BurnIntensity`)) _returnvalue)
      (`/Game/Statuses/BP_Status.ApplyStatus` _returnvalue _asbp_player_pawn _asbp_player_controller))))

(fn `UserConstructionScript`)