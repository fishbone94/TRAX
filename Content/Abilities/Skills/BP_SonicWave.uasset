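; BP_SonicWave is a skill that fires a forward wave from the caster to knock back other player pawns.
; SkillEffect runs a multi-sphere trace on the Camera channel along the caster's facing, sized by skill range and wave radius, with debug drawing enabled.
; Each hit spawns an emitter and sound.
; Hit BP_PlayerPawns launch away from the caster; velocity is the unnormalized offset times KnockbackPower, so it grows with distance.
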(event `self.SkillEffect`
  (params (PlayerReference :type "/Game/Core/BP_PlayerController Object Reference"))
  (bind (_skillinfo_skillname _skillinfo_icon _skillinfo_description _skillinfo_element _skillinfo_range) (break `/Game/Abilities/Skills/STR_SkillInfo` (`self.SkillInfo`)))
  (bind _asbp_player_pawn (cast `/Game/Player/BP_PlayerPawn` (`Controller.K2_GetPawn` PlayerReference)))
  (bind _returnvalue (`self.K2_GetActorLocation` _asbp_player_pawn))
  (bind (_outhits _returnvalue_2) (`KismetSystemLibrary.SphereTraceMulti` _returnvalue (+ _returnvalue (* (`self.GetActorForwardVector` _asbp_player_pawn) _skillinfo_range)) (`self.WaveRadius`) "TraceTypeQuery2" false (`|MakeArray` _asbp_player_pawn) "ForDuration" true (struct :`R` 1.0 :`A` 1.0) (struct :`G` 1.0 :`A` 1.0) 2.0))
  (if _returnvalue_2
    (for _array_element _outhits
      (bind (_bblockinghit _binitialoverlap _time _location _impactpoint _normal _impactnormal _physmat _hitactor) (`GameplayStatics.BreakHitResult` _array_element))
      (`GameplayStatics.SpawnEmitterAtLocation` null _location)
      (`GameplayStatics.PlaySoundAtLocation` null _location)
      (if (`KismetMathLibrary.ClassIsChildOf` (`GameplayStatics.GetObjectClass` _hitactor) "/Game/Player/BP_PlayerPawn.BP_PlayerPawn_C")
        (bind _asbp_player_pawn_2 (cast `/Game/Player/BP_PlayerPawn` _hitactor))
        (`Character.LaunchCharacter` _asbp_player_pawn_2 (* (- (`self.K2_GetActorLocation` _hitactor) (`self.K2_GetActorLocation` _asbp_player_pawn)) (`self.KnockbackPower`)) true true)))))

(fn `UserConstructionScript`
  (`parent.UserConstructionScript`))