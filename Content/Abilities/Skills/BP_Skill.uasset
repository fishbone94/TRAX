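; Base skill Blueprint that gates casting on cooldown and casting state, reporting cast start and end to the player controller.
; OnSkillCast runs SkillEffect, a placeholder printing the skill name, then completes immediately; child skills are meant to override this.
; Completion starts the cooldown, and with a valid Hotkey widget, a Timeline resized to the skill's cooldown drives its radial material and countdown text.
; Timeline completion clears the cooldown and restores the hotkey unless deactivated.
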(event `self.ReceiveBeginPlay`
  (bind _asbp_player_controller (cast `/Game/Core/BP_PlayerController` (`GameplayStatics.GetPlayerController` 0)))
  (set `self.PlayerReference` _asbp_player_controller))

(event `AttemptUseSkill`
  (params (PlayerController :type "/Game/Core/BP_PlayerController Object Reference"))
  ;[1 1 1] Attempt to use skill
  (set `self.PlayerReference` PlayerController)
  (if (and (not (`self.OnCooldown`)) (not (`self.IsCasting`)) (not (`/Game/Core/BP_PlayerController.IsCasting` (`self.PlayerReference`))))
    (`self.OnSkillCast`)))

(event `SkillEffect`
  (`KismetSystemLibrary.PrintString` (`KismetTextLibrary.Conv_TextToString` (`|FormatText` "Casting {Name}" (`.SkillName_2_6BACF43447DC0849046D5F964D15CF9A` (break `/Game/Abilities/Skills/STR_SkillInfo` (`self.SkillInfo`))))) true true (struct :`G` 0.66 :`B` 1.0 :`A` 1.0) 2.0))

(event `OnSkillCast`
  ;[1 1 1] Skill mechanic
  (set `self.IsCasting` true)
  (`/Game/Core/BP_PlayerController.BeginSkillCast` (`self.PlayerReference`) self)
  ;;[1 0.23 0.23] Override in Child
  (`self.SkillEffect`)
  (`self.OnCastCompleted`))

(event `OnCastCompleted`
  (bind _hotkey (`self.Hotkey`))
  (bind _hotkey_2 (`self.Hotkey`))
  (bind _cooldowntimeline (`self.CooldownTimeline`))
  (bind ((`Cooldown_10_6A42F6274C90D57A0F6B18B96384701A` _cooldown)) (break `/Game/Abilities/Skills/STR_SkillInfo` (`self.SkillInfo`)))
  (bind _returnvalue (`TimelineComponent.GetPlaybackPosition` _cooldowntimeline))
  (bind _returnvalue_2 (`TimelineComponent.GetTimelineLength` _cooldowntimeline))
  (bind _cooldowntext (`/Game/UI/WBP_SkillHotkey.CooldownText` _hotkey))
  (bind _returnvalue_3 (- _returnvalue_2 _returnvalue))
  (`/Game/Core/BP_PlayerController.EndSpellCast` (`self.PlayerReference`) self)
  (set `self.OnCooldown` true)
  (set `self.IsCasting` false)
  (`/Engine/EditorBlueprintResources/StandardMacros.IsValid` _hotkey
    (:`Is Valid`
      (`Widget.SetIsEnabled` (`/Game/UI/WBP_SkillHotkey.SkillButton` _hotkey) false)
      (`Image.SetColorAndOpacity` (`/Game/UI/WBP_SkillHotkey.SkillIcon` _hotkey) (struct :`R` 0.33 :`G` 0.33 :`B` 0.33 :`A` 1.0))
      (`MaterialInstanceDynamic.SetScalarParameterValue` (`/Game/UI/WBP_SkillHotkey.CooldownMaterial` _hotkey) "Percent" 1.0)
      (`Widget.SetVisibility` (`/Game/UI/WBP_SkillHotkey.CooldownImage` _hotkey) "HitTestInvisible")
      (`TextBlock.SetText` _cooldowntext (`KismetTextLibrary.Conv_DoubleToText` _cooldown "HalfToEven" true 1 324 0 0))
      (`Widget.SetVisibility` _cooldowntext "Visible")
      (`TimelineComponent.SetTimelineLength` (`self.CooldownTimeline`) _cooldown)
      (`Timeline|CooldownTimeline` :!via `PlayFromStart`
        (:`Update`
          (`/Engine/EditorBlueprintResources/StandardMacros.IsValid` _hotkey_2
            (:`Is Valid`
              (`MaterialInstanceDynamic.SetScalarParameterValue` (`/Game/UI/WBP_SkillHotkey.CooldownMaterial` _hotkey_2) "Percent" (- 1.0 (/ _returnvalue _returnvalue_2)))
              (`TextBlock.SetText` (`/Game/UI/WBP_SkillHotkey.CooldownText` _hotkey_2) (`KismetTextLibrary.Conv_DoubleToText` _returnvalue_3 "HalfToEven" false 1 324 0 (select `bool` (> _returnvalue_3 0.0) :`false` 1))))))
        (:`Finished`
          (`self.OnCooldownExpired`))))))

(event `OnCooldownExpired`
  (bind _hotkey (`self.Hotkey`))
  (set `self.OnCooldown` false)
  (`/Engine/EditorBlueprintResources/StandardMacros.IsValid` _hotkey
    (:`Is Valid`
      (if (not (`/Game/UI/WBP_SkillHotkey.IsDeactivated` _hotkey))
        (`Widget.SetIsEnabled` (`/Game/UI/WBP_SkillHotkey.SkillButton` _hotkey) true)
        (`Image.SetColorAndOpacity` (`/Game/UI/WBP_SkillHotkey.SkillIcon` _hotkey) (struct :`R` 1.0 :`G` 1.0 :`B` 1.0 :`A` 1.0)))
      (`Widget.SetVisibility` (`/Game/UI/WBP_SkillHotkey.CooldownImage` _hotkey) "Hidden")
      (`Widget.SetVisibility` (`/Game/UI/WBP_SkillHotkey.CooldownText` _hotkey) "Hidden"))))

(fn `UserConstructionScript`)