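; BP_Agility is a skill Blueprint that temporarily boosts the player's jump height.
; SkillEffect casts the given player's controlled pawn to BP_PlayerPawn and multiplies its CharacterMovement JumpZVelocity by JumpMultiplier.
; A one-shot timer set to the skill's duration then fires EndSkillEffect, which divides the velocity by the same multiplier to undo the boost.
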(event `self.SkillEffect`
  (params (PlayerReference :type "/Game/Core/BP_PlayerController Object Reference"))
  (bind (_skillinfo_skillname _skillinfo_icon _skillinfo_description _skillinfo_element _skillinfo_range _skillinfo_damage _skillinfo_duration) (break `/Game/Abilities/Skills/STR_SkillInfo` (`self.SkillInfo`)))
  (bind _asbp_player_pawn (cast `/Game/Player/BP_PlayerPawn` (`Controller.K2_GetPawn` PlayerReference)))
  (bind _charactermovement (`Character.CharacterMovement` _asbp_player_pawn))
  (set `CharacterMovementComponent.JumpZVelocity` (* (`CharacterMovementComponent.JumpZVelocity` _charactermovement) (`self.JumpMultiplier`)) _charactermovement)
  (`KismetSystemLibrary.K2_SetTimerDelegate` (delegate `EndSkillEffect`) _skillinfo_duration))

(event `EndSkillEffect`
  (bind _charactermovement (`Character.CharacterMovement` (stale `self.SkillEffect` _asbp_player_pawn)))
  (set `CharacterMovementComponent.JumpZVelocity` (/ (`CharacterMovementComponent.JumpZVelocity` _charactermovement) (`self.JumpMultiplier`)) _charactermovement))

(fn `UserConstructionScript`
  (`parent.UserConstructionScript`))