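; BP_SmokeBomb is a skill that launches a smoke bomb item from the player's pawn.
; Its SkillEffect event casts the controlled pawn to BP_PlayerPawn, then spawns BP_SmokeBombItem slightly above and ahead of it, regardless of collision.
; The spawn rotation follows the camera's pitch and yaw, with a randomized roll.
; Any motion or smoke behavior is left to the spawned item.
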(event `self.SkillEffect`
  (params (PlayerReference :type "/Game/Core/BP_PlayerController Object Reference"))
  (bind _asbp_player_pawn (cast `/Game/Player/BP_PlayerPawn` (`Controller.K2_GetPawn` PlayerReference)))
  (`|SpawnActorFromClass` "/Game/Abilities/Skills/SkillObjects/BP_SmokeBombItem.BP_SmokeBombItem_C" (`KismetMathLibrary.MakeTransform` (+ (`KismetMathLibrary.MakeVector` (.x (`self.K2_GetActorLocation` _asbp_player_pawn)) (.y (`self.K2_GetActorLocation` _asbp_player_pawn)) (+ (.z (`self.K2_GetActorLocation` _asbp_player_pawn)) 50.0)) (* (`self.GetActorForwardVector` _asbp_player_pawn) 150.0)) (`KismetMathLibrary.MakeRotator` (`KismetMathLibrary.RandomFloatInRange` -45.0 45.0) (.pitch (`SceneComponent.K2_GetComponentRotation` (`/Game/Player/BP_PlayerPawn.Camera` _asbp_player_pawn))) (.yaw (`SceneComponent.K2_GetComponentRotation` (`/Game/Player/BP_PlayerPawn.Camera` _asbp_player_pawn))))) "AlwaysSpawn" "OverrideRootScale"))

(fn `UserConstructionScript`
  (`parent.UserConstructionScript`))