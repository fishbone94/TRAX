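; Quick Attack skill that temporarily boosts the player's attack speed.
; SkillEffect casts the given player's controlled pawn to BP_PlayerPawn and adds AttackSpeedBonus to its AttackSpeed.
; A one-shot timer set to the duration in SkillInfo then fires EndSkillEffect, which subtracts the same bonus from that pawn.
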(event `self.SkillEffect`
  (params (PlayerReference :type "/Game/Core/BP_PlayerController Object Reference"))
  (bind (_skillinfo_skillname _skillinfo_icon _skillinfo_description _skillinfo_element _skillinfo_range _skillinfo_damage _skillinfo_duration) (break `/Game/Abilities/Skills/STR_SkillInfo` (`self.SkillInfo`)))
  (bind _asbp_player_pawn (cast `/Game/Player/BP_PlayerPawn` (`Controller.K2_GetPawn` PlayerReference)))
  (set `/Game/Player/BP_PlayerPawn.AttackSpeed` (+ (`/Game/Player/BP_PlayerPawn.AttackSpeed` _asbp_player_pawn) (`self.AttackSpeedBonus`)) _asbp_player_pawn)
  (`KismetSystemLibrary.K2_SetTimerDelegate` (delegate `EndSkillEffect`) _skillinfo_duration))

(event `EndSkillEffect`
  (set `/Game/Player/BP_PlayerPawn.AttackSpeed` (- (`/Game/Player/BP_PlayerPawn.AttackSpeed` (stale `self.SkillEffect` _asbp_player_pawn)) (`self.AttackSpeedBonus`)) (stale `self.SkillEffect` _asbp_player_pawn)))

(fn `UserConstructionScript`
  (`parent.UserConstructionScript`))