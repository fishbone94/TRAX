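; BP_EnchantFire is a skill that temporarily applies a fire enchantment to the player's weapon.
; SkillEffect casts the controlled pawn of the passed player reference to BP_PlayerPawn and sets its WeaponEnchanted enum.
; A one-shot timer lasting the SkillInfo duration then calls EndSkillEffect, which switches the enum to another value to end the enchantment, with debug prints marking both changes.
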(event `self.SkillEffect`
  (params (PlayerReference :type "/Game/Core/BP_PlayerController Object Reference"))
  (bind (_skillinfo_skillname _skillinfo_icon _skillinfo_description _skillinfo_element _skillinfo_range _skillinfo_damage _skillinfo_duration) (break `/Game/Abilities/Skills/STR_SkillInfo` (`self.SkillInfo`)))
  (bind _asbp_player_pawn (cast `/Game/Player/BP_PlayerPawn` (`Controller.K2_GetPawn` PlayerReference)))
  (set `/Game/Player/BP_PlayerPawn.WeaponEnchanted` "NewEnumerator0" _asbp_player_pawn)
  (`KismetSystemLibrary.PrintString` "Enchant Fire" true true (struct :`R` 1.0 :`G` 0.048928 :`A` 1.0))
  (`KismetSystemLibrary.K2_SetTimerDelegate` (delegate `EndSkillEffect`) _skillinfo_duration))

(event `EndSkillEffect`
  (set `/Game/Player/BP_PlayerPawn.WeaponEnchanted` "NewEnumerator6" (stale `self.SkillEffect` _asbp_player_pawn))
  (`KismetSystemLibrary.PrintString` "End Enchantment" true true (struct :`R` 1.0 :`G` 0.032916 :`A` 1.0)))

(fn `UserConstructionScript`
  (`parent.UserConstructionScript`))