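; BP_FireWalker is a player skill that leaves a trail of fire behind the player pawn for the skill's duration.
; SkillEffect casts the controlled pawn to BP_PlayerPawn, then starts a looping tick timer and a one-shot timer set by SkillInfo.Duration.
; Each tick spawns a BP_FireTrail at the pawn's mesh location, only while it is moving on ground.
; When the duration expires, EndSkillEffect clears both timers.
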(event `self.SkillEffect`
  (params (PlayerReference :type "/Game/Core/BP_PlayerController Object Reference"))
  (bind (_skillinfo_skillname _skillinfo_icon _skillinfo_description _skillinfo_element _skillinfo_range _skillinfo_damage _skillinfo_duration) (break `/Game/Abilities/Skills/STR_SkillInfo` (`self.SkillInfo`)))
  (bind _asbp_player_pawn (cast `/Game/Player/BP_PlayerPawn` (`Controller.K2_GetPawn` PlayerReference)))
  (bind _returnvalue (`KismetSystemLibrary.K2_SetTimerDelegate` (delegate `SkillTick`) 0.25 true))
  (bind _returnvalue_2 (`KismetSystemLibrary.K2_SetTimerDelegate` (delegate `EndSkillEffect`) _skillinfo_duration)))

(event `SkillTick`
  (if (`NavMovementComponent.IsMovingOnGround` (`Character.CharacterMovement` (stale `self.SkillEffect` _asbp_player_pawn)))
    (`|SpawnActorFromClass` "/Game/Abilities/Skills/SkillObjects/BP_FireTrail.BP_FireTrail_C" (`KismetMathLibrary.MakeTransform` (`SceneComponent.K2_GetComponentLocation` (`Character.Mesh` (stale `self.SkillEffect` _asbp_player_pawn)))) "AlwaysSpawn" "OverrideRootScale")))

(event `EndSkillEffect`
  (`KismetSystemLibrary.K2_ClearAndInvalidateTimerHandle` (stale `self.SkillEffect` _returnvalue))
  (`KismetSystemLibrary.K2_ClearAndInvalidateTimerHandle` (stale `self.SkillEffect` _returnvalue_2)))

(fn `UserConstructionScript`
  (`parent.UserConstructionScript`))