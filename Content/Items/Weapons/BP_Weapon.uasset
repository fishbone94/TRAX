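; BP_Weapon is a weapon Blueprint that performs a sphere-sweep attack from the player pawn, driven by its WeaponInfo data.
; On BeginPlay it caches the player pawn as BP_PlayerPawn.
; Attack runs a multi sphere trace forward on the Camera channel, sized by Range and Cleave, with timed debug drawing.
; Each hit gets the configured VFX, sound and damage, with the player as damage causer.
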(event `self.ReceiveBeginPlay`
  (bind _asbp_player_pawn (cast `/Game/Player/BP_PlayerPawn` (`GameplayStatics.GetPlayerPawn` 0)))
  (set `self.CharacterReference` _asbp_player_pawn))

(event `Attack`
  (bind (_weaponinfo_attacktype _weaponinfo_damage _weaponinfo_range _weaponinfo_cleave) (break `/Game/Items/Weapons/STR_WeaponInfo` (`self.WeaponInfo`)))
  (bind _characterreference (`self.CharacterReference`))
  (bind ((`Damage_5_CEC76266406693B1519054AC2D7BAD91` _damage) (`Cleave_42_73688D354C1E8CC2922F13873B893201` _cleave) (`RightHandWeapon_38_5DCEAACE4AFD931F57D2E4A6C2A7E162` _righthandweapon) (`RightHandSheath_36_233E74664336C81B220BC1B431E8BF1D` _righthandsheath) (`LeftHandWeapon_39_6FA1F7AE4F0607FA2B325E8F6CAFD7E3` _lefthandweapon) (`LeftHandSheath_37_593F6D6B433CBF88F378359FC8734501` _lefthandsheath) (`HitVFX_25_96ADA5284F43D85110C98D8C42699DF3` _hitvfx) (`HitSFX_28_89B18C484197A5E58244F0AE8B4EAACA` _hitsfx)) (break `/Game/Items/Weapons/STR_WeaponInfo` (`self.WeaponInfo`)))
  (bind _returnvalue (`self.K2_GetActorLocation` _characterreference))
  (bind (_outhits _returnvalue_2) (`KismetSystemLibrary.SphereTraceMulti` _returnvalue (+ _returnvalue (* (`self.GetActorForwardVector` _characterreference) _weaponinfo_range)) _weaponinfo_cleave "TraceTypeQuery2" false (`|MakeArray` _characterreference :!type "Actor Object Reference") "ForDuration" true (struct :`R` 1.0 :`A` 1.0) (struct :`G` 1.0 :`A` 1.0) 2.0))
  (if _returnvalue_2
    (for _array_element _outhits
      (bind (_bblockinghit _binitialoverlap _time _location _impactpoint _normal _impactnormal _physmat _hitactor) (`GameplayStatics.BreakHitResult` _array_element))
      (`GameplayStatics.SpawnEmitterAtLocation` _hitvfx _location)
      (`GameplayStatics.PlaySoundAtLocation` _hitsfx _location)
      (`GameplayStatics.ApplyDamage` _hitactor _damage null (`self.CharacterReference`)))))

(fn `UserConstructionScript`
  (`parent.UserConstructionScript`))