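; Consumable bear trap that the player places in the world on use.
; UseConsumable line-traces on the Visibility channel from the player's camera, out to the pawn's RaycastLength.
; It spawns a BP_BearTrapItem slightly below the hit location with zero rotation and turns off its CanBeInteracted flag.
; The trace result is not checked, so the spawn runs even when nothing is hit.
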(event `self.UseConsumable`
  (params (PlayerPawn :type "/Game/Player/BP_PlayerPawn Object Reference") (PlayerController :type "/Game/Core/BP_PlayerController Object Reference"))
  (bind _camera (`/Game/Player/BP_PlayerPawn.Camera` PlayerPawn))
  (bind _returnvalue (`SceneComponent.K2_GetComponentLocation` _camera))
  (bind _outhit (`KismetSystemLibrary.LineTraceSingle` :`Start` _returnvalue :`End` (+ _returnvalue (* (`KismetMathLibrary.GetForwardVector` (`SceneComponent.K2_GetComponentRotation` _camera)) (`/Game/Player/BP_PlayerPawn.RaycastLength` PlayerPawn))) :`TraceChannel` "TraceTypeQuery1" :`DrawTime` 1.0))
  (bind _returnvalue_2 (`|SpawnActorFromClass` "/Game/Items/Consumables/BP_BearTrapItem.BP_BearTrapItem_C" (`KismetMathLibrary.MakeTransform` (`KismetMathLibrary.MakeVector` (.x (`.Location` (`GameplayStatics.BreakHitResult` _outhit))) (.y (`.Location` (`GameplayStatics.BreakHitResult` _outhit))) (- (.z (`.Location` (`GameplayStatics.BreakHitResult` _outhit))) 6.0))) "AdjustIfPossibleButAlwaysSpawn" "OverrideRootScale"))
  (set `/Game/Items/BP_InteractItem.CanBeInteracted` false _returnvalue_2))

(fn `UserConstructionScript`
  (`parent.UserConstructionScript`))