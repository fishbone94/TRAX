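; BP_BearTrapItem is a trap that damages and cripples a player who steps into it, then destroys itself.
; On a sphere overlap, the server checks for a BP_PlayerPawn, then spawns BP_Burning and, after a short delay, BP_Cripple.
; Each status actor gets a status info struct built from the trap's variables and is applied to that player.
; The Burning status takes its intensity from the Bleeding variable.
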(event `self.ReceiveActorBeginOverlap`
  (params (OtherActor :type "Actor Object Reference")))

(event `self.Sphere.OnComponentBeginOverlap`
  (params (OverlappedComponent :type "PrimitiveComponent Object Reference") (OtherActor :type "Actor Object Reference") (OtherComp :type "PrimitiveComponent Object Reference") (OtherBodyIndex :type Integer) (bFromSweep :type Boolean) (SweepResult :type "HitResult Structure (by ref)"))
  (`/Engine/EditorBlueprintResources/ActorMacros.Switch Has Authority`
    (:`Authority`
      (if (`KismetMathLibrary.ClassIsChildOf` (`GameplayStatics.GetObjectClass` OtherActor) "/Game/Player/BP_PlayerPawn.BP_PlayerPawn_C")
        (bind _asbp_player_pawn (cast `/Game/Player/BP_PlayerPawn` OtherActor))
        (bind _asbp_player_controller (cast `/Game/Core/BP_PlayerController` (`Pawn.GetController` _asbp_player_pawn)))
        (`KismetSystemLibrary.PrintString` "Triggered")
        (bind _returnvalue (`|SpawnActorFromClass` "/Game/Statuses/BP_Burning.BP_Burning_C" (`self.GetTransform`) "AlwaysSpawn" "OverrideRootScale"))
        (set `/Game/Statuses/BP_Status.StatusInfo` (make `/Game/Statuses/STR_StatusInfo` "Burning" "/Game/UI/Assets/T_FlameNova.T_FlameNova" "" "NewEnumerator2" (`self.Duration`) (`self.Bleeding`)) _returnvalue)
        (`/Game/Statuses/BP_Status.ApplyStatus` _returnvalue _asbp_player_pawn _asbp_player_controller)
        (`KismetSystemLibrary.Delay` 0.2)
        (bind _returnvalue_2 (`|SpawnActorFromClass` "/Game/Statuses/BP_Cripple.BP_Cripple_C" (`self.GetTransform`) "AlwaysSpawn" "OverrideRootScale"))
        (set `/Game/Statuses/BP_Status.StatusInfo` (make `/Game/Statuses/STR_StatusInfo` "Crippled" "/Game/UI/Assets/T_Cleanse.T_Cleanse" "" "NewEnumerator2" (`self.Duration`) (`self.Cripple`)) _returnvalue_2)
        (`/Game/Statuses/BP_Status.ApplyStatus` _returnvalue_2 _asbp_player_pawn _asbp_player_controller)
        (`self.K2_DestroyActor`)))))

(fn `UserConstructionScript`
  (`parent.UserConstructionScript`))