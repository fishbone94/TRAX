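; Player character with third-person-style movement, stamina-based sprint and dodge, combo melee, and right-hand weapon equipping.
; Inputs call WantsTo events that check state before actions; looping timers drain and regenerate stamina, and dodges launch by velocity.
; Primary attacks buffer input across three montages; secondary attack only prints.
; A per-tick camera trace sets LookingAt; equipment snaps to weapon-defined hand or sheath sockets, dropping replaced items.
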(event `InputAction|SecondaryAttack`
  (params (Key :type "Key Structure" :default "AnyKey"))
  ;[1 1 1] Secondary Attack
  (:`Pressed`
    (`self.WantsToSecondaryAttack`))
  (:`Released`
    (`self.WantsToStopSecondaryAttack`)))

(event `self.ReceiveBeginPlay`)

(event `InputAction|PrimaryAttack`
  (params (Key :type "Key Structure" :default "AnyKey"))
  ;[1 1 1] Combo Attacks
  (:`Pressed`
    (`self.WantsToPrimaryAttack`)))

(event `ResetCombo`
  ;[1 1 1] Combo Attacks
  (set `self.ComboCounter` 0)
  (set `self.SaveAttack` false)
  (set `self.IsAttacking` false))

(event `SaveComboAttack`
  ;[1 1 1] Combo Attacks
  (if (`self.SaveAttack`)
    (set `self.SaveAttack` false)
    (switch `int` (`self.ComboCounter`) :!label _label
      (:`0`
        (set `self.ComboCounter` 1)
        (`self.ComboMontage_1`))
      (:`1`
        (set `self.ComboCounter` 2)
        (`self.ComboMontage_2`))
      (:`2`
        (set `self.ComboCounter` 3)
        (`self.ComboMontage_3`)))))

(event `WantsToSecondaryAttack`
  ;[1 1 1] Secondary Attack
  (if (and (not (`NavMovementComponent.IsFalling` (`self.CharacterMovement`))) (not (`self.IsDodging`)) (`self.HasWeaponAttached`) (not (`self.HasWeaponSheathed`)))
    (set `self.IsSecondaryAttacking` true)
    (`KismetSystemLibrary.PrintString` "Secondary")))

(event `self.ReceiveTick`
  (params (DeltaSeconds :type "Float (single-precision)"))
  (bind _camera (`self.Camera`))
  (bind _returnvalue (`SceneComponent.K2_GetComponentLocation` _camera))
  (`|ExecutionSequence`
    (:`then_0`
      ;[1 1 1] Raycast from camera
      (bind _outhit (`KismetSystemLibrary.LineTraceSingle` :`Start` _returnvalue :`End` (+ _returnvalue (* (`KismetMathLibrary.GetForwardVector` (`SceneComponent.K2_GetComponentRotation` _camera)) (`self.RaycastLength`))) :`TraceChannel` "TraceTypeQuery1" :`DrawTime` 1.0))
      (set `self.LookingAt` (`.HitActor` (`GameplayStatics.BreakHitResult` _outhit))))))

(event `WantsToPrimaryAttack`
  ;[1 1 1] Combo Attacks
  (if (and (not (`NavMovementComponent.IsFalling` (`self.CharacterMovement`))) (not (`self.IsDodging`)) (`self.HasWeaponAttached`) (not (`self.HasWeaponSheathed`)))
    (if (`self.IsAttacking`)
      (set `self.SaveAttack` true)
      (else
        (set `self.IsAttacking` true)
        (goto _label)))))

(event `InputAction|Crouch`
  (params (Key :type "Key Structure" :default "AnyKey"))
  ;[1 1 1] Inputs
  (:`Pressed`
    (`self.Crouch`)
    (set `self.IsCrouching` true))
  (:`Released`
    (`self.UnCrouch`)
    (set `self.IsCrouching` false)))

(event `WantsToStopSecondaryAttack`
  ;[1 1 1] Secondary Attack
  (if (`self.IsSecondaryAttacking`)
    (set `self.IsSecondaryAttacking` false)
    (`KismetSystemLibrary.PrintString` "Stop Secondary")))

(event `ComboMontage_1`
  ;[1 1 1] Combo Attacks
  (`AnimInstance.Montage_Play` (`SkeletalMeshComponent.GetAnimInstance` (`self.Mesh`)) "/Game/Player/Mannequin/Animations/SwordShield/AM_Combo_1.AM_Combo_1" 1.0 "MontageLength" 0.0))

(event `InputAction|Jump`
  (params (Key :type "Key Structure" :default "AnyKey"))
  ;[1 1 1] Inputs
  (:`Pressed`
    (`self.Jump`))
  (:`Released`
    (`self.StopJumping`)))

(event `ComboMontage_2`
  ;[1 1 1] Combo Attacks
  (`AnimInstance.Montage_Play` (`SkeletalMeshComponent.GetAnimInstance` (`self.Mesh`)) "/Game/Player/Mannequin/Animations/SwordShield/AM_Combo_2.AM_Combo_2" 1.0 "MontageLength" 0.0))

(event `WantsToSprint`
  ;[1 1 1] Sprint
  (if (and (>= (`self.CurrentStamina`) 100.0) (not (`NavMovementComponent.IsFalling` (`self.CharacterMovement`))) (not (`self.IsDodging`)) (not (`self.IsCrouching`)))
    (set `self.IsSprinting` true)
    (`self.BeginSprint`)
    (bind _returnvalue (`KismetSystemLibrary.K2_SetTimerDelegate` (delegate `DegenStamina`) 0.1 true))
    (`KismetSystemLibrary.K2_ClearAndInvalidateTimerHandle` (stale `WantsToWalk` _returnvalue))
    (`KismetSystemLibrary.K2_ClearAndInvalidateTimerHandle` (stale `DegenStamina` _returnvalue))))

(event `InputAction|Sprint`
  (params (Key :type "Key Structure" :default "AnyKey"))
  ;[1 1 1] Inputs
  (:`Pressed`
    (`self.WantsToSprint`))
  (:`Released`
    (`self.WantsToWalk`)))

(event `ComboMontage_3`
  ;[1 1 1] Combo Attacks
  (`AnimInstance.Montage_Play` (`SkeletalMeshComponent.GetAnimInstance` (`self.Mesh`)) "/Game/Player/Mannequin/Animations/SwordShield/AM_Combo_3.AM_Combo_3" 1.0 "MontageLength" 0.0))

(event `InputAction|Dodge`
  (params (Key :type "Key Structure" :default "AnyKey"))
  ;[1 1 1] Inputs
  (:`Pressed`
    (`self.WantsToDodge` (`self.ForwardSpeed`) (`self.RightSpeed`))))

(event `DegenStamina`
  ;[1 1 1] Degen Stamina
  (if (<= (`self.CurrentStamina`) 0.0)
    (set `self.IsSprinting` false)
    (`self.BeginWalk`)
    (`KismetSystemLibrary.K2_ClearAndInvalidateTimerHandle` (stale `WantsToSprint` _returnvalue))
    (bind _returnvalue (`KismetSystemLibrary.K2_SetTimerDelegate` (delegate `RegenStamina`) 0.1 true))
    (else
      (`self.ChangeStamina` -10.0))))

(event `DrawWeaponMontage`
  ;[1 1 1] Draw/Sheath Weapon
  (`AnimInstance.Montage_Play` (`SkeletalMeshComponent.GetAnimInstance` (`self.Mesh`)) "/Game/Player/Mannequin/Animations/SwordShield/AM_DrawWeapon.AM_DrawWeapon" 1.0 "MontageLength" 0.0))

(event `InputAction|ToggleWeapon`
  (params (Key :type "Key Structure" :default "AnyKey"))
  ;[1 1 1] Draw/Sheath Weapon
  (:`Pressed`
    (`self.WantsToToggleWeapon`)))

(event `WantsToToggleWeapon`
  ;[1 1 1] Draw/Sheath Weapon
  (`/Engine/EditorBlueprintResources/StandardMacros.IsValid` (`self.RightHandWeapon`)
    (:`Is Valid`
      (if (`self.HasWeaponSheathed`)
        (`self.DrawWeaponMontage`)
        (else
          (`self.SheathWeaponMontage`))))))

(event `WantsToWalk`
  ;[1 1 1] Walk
  (set `self.IsSprinting` false)
  (`self.BeginWalk`)
  (bind _returnvalue (`KismetSystemLibrary.K2_SetTimerDelegate` (delegate `RegenStamina`) 0.1 true))
  (`KismetSystemLibrary.K2_ClearAndInvalidateTimerHandle` (stale `WantsToSprint` _returnvalue)))

(event `SheathWeaponMontage`
  ;[1 1 1] Draw/Sheath Weapon
  (`AnimInstance.Montage_Play` (`SkeletalMeshComponent.GetAnimInstance` (`self.Mesh`)) "/Game/Player/Mannequin/Animations/SwordShield/AM_SheathWeapon.AM_SheathWeapon" 1.0 "MontageLength" 0.0))

(event `DrawWeapon`
  ;[1 1 1] Draw/Sheath Weapon
  (bind _asbp_weapon (cast `/Game/Items/Weapons/BP_Weapon` (`self.RightHandWeapon`)))
  (`self.K2_AttachToComponent` (`self.RightHandWeapon`) (`self.Mesh`) (`.RightHandWeapon_38_5DCEAACE4AFD931F57D2E4A6C2A7E162` (break `/Game/Items/Weapons/STR_WeaponInfo` (`/Game/Items/Weapons/BP_Weapon.WeaponInfo` _asbp_weapon))) "SnapToTarget" "SnapToTarget" "SnapToTarget" true)
  (set `self.HasWeaponSheathed` false)
  (set `self.HasWeaponAttached` true))

(event `RegenStamina`
  ;[1 1 1] Regen Stamina
  (if (>= (`self.CurrentStamina`) (`self.MaxStamina`))
    (`KismetSystemLibrary.K2_ClearAndInvalidateTimerHandle` (stale `WantsToWalk` _returnvalue))
    (`KismetSystemLibrary.K2_ClearAndInvalidateTimerHandle` (stale `DegenStamina` _returnvalue))
    (else
      (`self.ChangeStamina` 5.0))))

(event `SheathWeapon`
  ;[1 1 1] Draw/Sheath Weapon
  (bind _asbp_weapon (cast `/Game/Items/Weapons/BP_Weapon` (`self.RightHandWeapon`)))
  (`self.K2_AttachToComponent` (`self.RightHandWeapon`) (`self.Mesh`) (`.RightHandSheath_36_233E74664336C81B220BC1B431E8BF1D` (break `/Game/Items/Weapons/STR_WeaponInfo` (`/Game/Items/Weapons/BP_Weapon.WeaponInfo` _asbp_weapon))) "SnapToTarget" "SnapToTarget" "SnapToTarget" true)
  (set `self.HasWeaponSheathed` true)
  (set `self.HasWeaponAttached` false))

(event `InputAxis|MouseX`
  (params (AxisValue :type "Float (single-precision)"))
  ;[1 1 1] Movement
  (if (!= AxisValue 0.0)
    (`self.AddControllerYawInput` AxisValue)))

(event `InputAxis|MoveForward`
  (params (AxisValue :type "Float (single-precision)"))
  ;[1 1 1] Movement
  (set `self.ForwardSpeed` (`KismetMathLibrary.Dot_VectorVector` (`self.GetVelocity`) (`self.GetActorForwardVector`)))
  (if (!= AxisValue 0.0)
    (`self.AddMovementInput` (`KismetMathLibrary.GetForwardVector` (`KismetMathLibrary.MakeRotator` 0.0 0.0 (.yaw (`self.GetControlRotation`)))) AxisValue)))

(event `InputAxis|MouseY`
  (params (AxisValue :type "Float (single-precision)"))
  ;[1 1 1] Movement
  (if (!= AxisValue 0.0)
    (`self.AddControllerPitchInput` AxisValue)))

(event `InputAxis|MoveRight`
  (params (AxisValue :type "Float (single-precision)"))
  ;[1 1 1] Movement
  (set `self.RightSpeed` (`KismetMathLibrary.Dot_VectorVector` (`self.GetVelocity`) (`self.GetActorRightVector`)))
  (if (!= AxisValue 0.0)
    (`self.AddMovementInput` (`KismetMathLibrary.GetRightVector` (`KismetMathLibrary.MakeRotator` 0.0 0.0 (.yaw (`self.GetControlRotation`)))) AxisValue)))

(event `DodgeBackward_Montage`
  (`AnimInstance.Montage_Play` (`SkeletalMeshComponent.GetAnimInstance` (`self.Mesh`)) "/Game/Player/Mannequin/Animations/Movement/AM_Dodge_Backward.AM_Dodge_Backward" 1.0 "MontageLength" 0.0))

(event `WantsToDodge`
  (params (ForwardSpeed :type "Float (double-precision)") (RightSpeed :type "Float (double-precision)"))
  ;[1 1 1] Dodge
  (if (and (>= (`self.CurrentStamina`) 200.0) (not (`NavMovementComponent.IsFalling` (`self.CharacterMovement`))) (not (`self.IsDodging`)))
    (if (> ForwardSpeed 10.0)
      (if (>= ForwardSpeed 350.0)
        (`self.DodgeForward_Montage`)
        (else
          (if (> RightSpeed 0.0)
            (`self.DodgeRight_Montage`)
            (else
              (`self.DodgeLeft_Montage`)))
          (`self.BeginDodge` :!label _label_2)))
      (elif (<= ForwardSpeed -350.0)
        (`self.DodgeBackward_Montage`)
        (elif (> RightSpeed 0.0)
          (`self.DodgeRight_Montage`)
          (goto _label_2)
          (else
            (`self.DodgeLeft_Montage`)
            (goto _label_2)))))))

(event `DodgeForward_Montage`
  (`AnimInstance.Montage_Play` (`SkeletalMeshComponent.GetAnimInstance` (`self.Mesh`)) "/Game/Player/Mannequin/Animations/Movement/AM_Dodge_Forward.AM_Dodge_Forward" 1.0 "MontageLength" 0.0))

(event `DodgeLeft_Montage`
  (`AnimInstance.Montage_Play` (`SkeletalMeshComponent.GetAnimInstance` (`self.Mesh`)) "/Game/Player/Mannequin/Animations/Movement/AM_Dodge_Left.AM_Dodge_Left" 1.0 "MontageLength" 0.0))

(event `self.ReceiveAnyDamage`
  (params (Damage :type "Float (single-precision)") (DamageType :type "DamageType Object Reference") (InstigatedBy :type "Controller Object Reference") (DamageCauser :type "Actor Object Reference"))
  ;[1 1 1] Take Damage Test
  (`self.ChangeHealth` (* Damage -1.0)))

(event `DodgeRight_Montage`
  (`AnimInstance.Montage_Play` (`SkeletalMeshComponent.GetAnimInstance` (`self.Mesh`)) "/Game/Player/Mannequin/Animations/Movement/AM_Dodge_Right.AM_Dodge_Right" 1.0 "MontageLength" 0.0))

(fn `AttachEquipment`
  (params (ItemInfo :type "/Game/Items/STR_ItemInfo Structure"))
  (bind (_itemtype _itemname _itemimage _itemclass _itemindex _itemslot) (break `/Game/Items/STR_ItemInfo` ItemInfo))
  (bind (_itemtype_2 _itemname_2 _itemimage_2 _itemclass_2 _itemindex_2 _itemslot_2) (break `/Game/Items/STR_ItemInfo` ItemInfo))
  (bind _righthandweapon (`self.RightHandWeapon`))
  (bind _righthandweapon_2 (`self.RightHandWeapon`))
  (if (`self.HasWeaponSheathed`)
    (switch `/Game/Items/ENUM_SlotType` _itemslot_2
      (:`NewEnumerator1`
        (`/Engine/EditorBlueprintResources/StandardMacros.IsValid` (`self.RightHandWeapon`)
          (:`Is Valid`
            (`self.SpawnDroppedItem` (`/Game/Items/BP_InteractItem.ItemInfo` _righthandweapon))
            (`self.K2_DestroyActor` _righthandweapon))
          (:`Is Not Valid`
            _))
        (bind _returnvalue (`|SpawnActorFromClass` _itemclass_2 (`self.GetTransform`) "AlwaysSpawn" "OverrideRootScale"))
        (bind _output_get (set `self.RightHandWeapon` _returnvalue))
        (bind _asbp_weapon (cast `/Game/Items/Weapons/BP_Weapon` _output_get))
        (`self.SetActorEnableCollision` _asbp_weapon false)
        (`self.K2_AttachToComponent` _asbp_weapon (`self.Mesh`) (`.RightHandSheath_36_233E74664336C81B220BC1B431E8BF1D` (break `/Game/Items/Weapons/STR_WeaponInfo` (`/Game/Items/Weapons/BP_Weapon.WeaponInfo` _asbp_weapon))) "SnapToTarget" "SnapToTarget" "SnapToTarget" true)
        (set `/Game/Items/BP_InteractItem.CanBeInteracted` false _asbp_weapon)))
    (else
      (switch `/Game/Items/ENUM_SlotType` _itemslot
        (:`NewEnumerator1`
          (`/Engine/EditorBlueprintResources/StandardMacros.IsValid` (`self.RightHandWeapon`)
            (:`Is Valid`
              (`self.SpawnDroppedItem` (`/Game/Items/BP_InteractItem.ItemInfo` _righthandweapon_2))
              (`self.K2_DestroyActor` _righthandweapon_2))
            (:`Is Not Valid`
              _))
          (bind _returnvalue_2 (`|SpawnActorFromClass` _itemclass (`self.GetTransform`) "AlwaysSpawn" "OverrideRootScale"))
          (bind _output_get_2 (set `self.RightHandWeapon` _returnvalue_2))
          (bind _asbp_weapon_2 (cast `/Game/Items/Weapons/BP_Weapon` _output_get_2))
          (`self.SetActorEnableCollision` _asbp_weapon_2 false)
          (`self.K2_AttachToComponent` _asbp_weapon_2 (`self.Mesh`) (`.RightHandWeapon_38_5DCEAACE4AFD931F57D2E4A6C2A7E162` (break `/Game/Items/Weapons/STR_WeaponInfo` (`/Game/Items/Weapons/BP_Weapon.WeaponInfo` _asbp_weapon_2))) "SnapToTarget" "SnapToTarget" "SnapToTarget" true)
          (set `/Game/Items/BP_InteractItem.CanBeInteracted` false _asbp_weapon_2))))))

(fn `BeginDodge`
  (bind _returnvalue (`self.GetVelocity`))
  (bind _dodgemultiplier (`self.DodgeMultiplier`))
  (set `self.CurrentStamina` (- (`self.CurrentStamina`) 200.0))
  (if (== (`KismetMathLibrary.VSize` _returnvalue) 0.0)
    ;[1 1 1] Dodge character backwards if not moving
    (`self.LaunchCharacter` (`KismetMathLibrary.MakeVector` (.x (* (`KismetMathLibrary.GetForwardVector` (`self.K2_GetActorRotation`)) (* (`self.WalkSpeed`) (`self.DodgeMultiplier`) -1.25))) (.y (* (`KismetMathLibrary.GetForwardVector` (`self.K2_GetActorRotation`)) (* (`self.WalkSpeed`) (`self.DodgeMultiplier`) -1.25)))))
    (else
      ;[1 1 1] Dodge character in direction they are moving
      (`self.LaunchCharacter` (`KismetMathLibrary.MakeVector` (* (.x _returnvalue) _dodgemultiplier) (* (.y _returnvalue) _dodgemultiplier)) false true)))
  (`KismetSystemLibrary.K2_SetTimer` self "EndDodge" 1.2))

(fn `BeginSprint`
  (set `CharacterMovementComponent.MaxWalkSpeed` (`self.SprintSpeed`) (`self.CharacterMovement`)))

(fn `BeginWalk`
  (set `CharacterMovementComponent.MaxWalkSpeed` (`self.WalkSpeed`) (`self.CharacterMovement`)))

(fn `ChangeHealth`
  (params (HealthInput :type "Float (double-precision)"))
  (set `self.CurrentHealth` (+ HealthInput (`self.CurrentHealth`)))
  (if (> (`self.CurrentHealth`) (`self.MaxHealth`))
    (set `self.CurrentHealth` (`self.MaxHealth`)))
  (if (<= (`self.CurrentHealth`) 0.0)
    (set `self.CurrentHealth` (`self.MaxHealth`))))

(fn `ChangeStamina`
  (params (StaminaInput :type "Float (double-precision)"))
  (set `self.CurrentStamina` (+ StaminaInput (`self.CurrentStamina`)))
  (if (> (`self.CurrentStamina`) (`self.MaxStamina`))
    (set `self.CurrentStamina` (`self.MaxStamina`))))

(fn `EndDodge`
  (set `self.IsDodging` false))

(fn `SpawnDroppedItem`
  (params (ItemInfo :type "/Game/Items/STR_ItemInfo Structure"))
  (bind _returnvalue (`|SpawnActorFromClass` (`.ItemClass_11_5381C432403ED9279DBC6996A4DDEDAB` (break `/Game/Items/STR_ItemInfo` ItemInfo)) (`KismetMathLibrary.MakeTransform` (+ (`self.K2_GetActorLocation`) (* (`self.GetActorForwardVector`) 200.0))) "AlwaysSpawn" "OverrideRootScale"))
  (`self.SetActorEnableCollision` _returnvalue true)
  (set `/Game/Items/BP_InteractItem.CanBeInteracted` true _returnvalue))

(fn `UnattachEquipment`
  (params (ItemInfo :type "/Game/Items/STR_ItemInfo Structure"))
  (switch `/Game/Items/ENUM_SlotType` (`.ItemSlot_17_EACED755413EF4800085B994CFBC485A` (break `/Game/Items/STR_ItemInfo` ItemInfo))
    (:`NewEnumerator1`
      (`self.K2_DestroyActor` (`self.RightHandWeapon`)))
    (:`NewEnumerator3`
      (`self.K2_DestroyActor` (`self.RightHandSheath`)))))

(fn `UserConstructionScript`)