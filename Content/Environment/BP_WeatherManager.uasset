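; Weather manager that runs a day-night cycle by rotating the level's directional light and refreshing the sky sphere.
; BeginPlay finds both actors, caches sun intensity and scales the start time into game-day seconds.
; Each tick advances elapsed time, sets sun pitch from a curve sampled at unwrapped elapsed hours, and derives the current day, hour and minute.
; A night-based sun intensity fade exists but is never called.
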(event `self.ReceiveBeginPlay`
  (`|ExecutionSequence`
    (:`then_0`
      (`self.GetSunAndSky`))
    (:`then_1`
      (`self.SetSunIntensity`))
    (:`then_2`
      (`self.SetElapsedTime`))))

(event `self.ReceiveTick`
  (params (DeltaSeconds :type "Float (single-precision)"))
  (`|ExecutionSequence`
    (:`then_0`
      (`self.UpdateElapsedTime`))
    (:`then_1`
      (`self.UpdateSunPosition`))
    (:`then_2`
      (`self.UpdateCurrentTime`))))

(fn `DetermineCurrentTime`
  (returns (Time :type "/Game/Environment/STR_Time Structure"))
  (bind _returnvalue (`self.GetFractionOfDay`))
  (return (make `/Game/Environment/STR_Time` (`KismetMathLibrary.FTrunc` _returnvalue) (`KismetMathLibrary.FTrunc` (* (mod _returnvalue 1.0) 24.0)) (`KismetMathLibrary.FTrunc` (mod (* _returnvalue 1440.0) 60.0)))))

(fn `DetermineIfNight`
  (returns (ReturnValue :type Boolean))
  (bind (_currenttime_days _currenttime_hours) (break `/Game/Environment/STR_Time` (`self.CurrentTime`)))
  (return (or (< _currenttime_hours (`self.SunUpTime`)) (>= _currenttime_hours (`self.SunDownTime`)))))

(fn `FadeSun`
  (bind _lightcomponent (`Light.LightComponent` (`self.Sun`)))
  (`LightComponent.SetIntensity` _lightcomponent (`KismetMathLibrary.FClamp` (+ (`LightComponentBase.Intensity` _lightcomponent) (* (`GameplayStatics.GetWorldDeltaSeconds`) (/ 24.0 (`self.SecondsPerDay`)) (`self.SunIntensity`) (select `bool` (`self.DetermineIfNight`) :`false` 1.0 :`true` -1.0 :!type "Float (single-precision)"))) 0.0 (`self.SunIntensity`))))

(fn `GetFractionOfDay`
  (returns (ReturnValue :type "Float (double-precision)"))
  (return (/ (`self.ElapsedTime`) (`self.SecondsPerDay`))))

(fn `GetSunAndSky`
  (`|ExecutionSequence`
    (:`then_0`
      (`/Engine/EditorBlueprintResources/StandardMacros.IsValid` (`self.Sun`)
        (:`Is Not Valid`
          (bind _outactors (`GameplayStatics.GetAllActorsOfClass` "/Script/Engine.DirectionalLight"))
          (set `self.Sun` (`KismetArrayLibrary.Array_Get` _outactors)))))
    (:`then_1`
      (`/Engine/EditorBlueprintResources/StandardMacros.IsValid` (`self.Sky`)
        (:`Is Not Valid`
          (bind _outactors_2 (`GameplayStatics.GetAllActorsOfClass` "/Engine/EngineSky/BP_Sky_Sphere.BP_Sky_Sphere_C"))
          (set `self.Sky` (`KismetArrayLibrary.Array_Get` _outactors_2)))))
    (:`then_2`
      (return))))

(fn `GetTimeAsSeconds`
  (params (Time :type "/Game/Environment/STR_Time Structure (by ref)"))
  (returns (ReturnValue :type Integer))
  (bind (_days _hours _minutes) (break `/Game/Environment/STR_Time` Time))
  (return (+ (* _days 86400) (* _hours 3600) (* _minutes 60))))

(fn `SetElapsedTime`
  (set `self.ElapsedTime` (* (`self.GetTimeAsSeconds` (`self.StartTime`)) (/ (`self.SecondsPerDay`) 86400.0))))

(fn `SetSunIntensity`
  (set `self.SunIntensity` (`LightComponentBase.Intensity` (`Light.LightComponent` (`self.Sun`)))))

(fn `UpdateCurrentTime`
  (set `self.CurrentTime` (`self.DetermineCurrentTime`)))

(fn `UpdateElapsedTime`
  (set `self.ElapsedTime` (+ (`self.ElapsedTime`) (`GameplayStatics.GetWorldDeltaSeconds`))))

(fn `UpdateSunPosition`
  (`SceneComponent.K2_SetRelativeRotation` (`Light.LightComponent` (`self.Sun`)) (`KismetMathLibrary.MakeRotator` 0.0 (`CurveFloat.GetFloatValue` (`self.DayNightCurve`) (* (`self.GetFractionOfDay`) 24.0)) 30.0) false false)
  (`/Engine/EngineSky/BP_Sky_Sphere.UpdateSunDirection` (`self.Sky`)))

(fn `UserConstructionScript`
  (set `self.SecondsPerDay` (* (`self.MinutesPerDay`) 60.0)))