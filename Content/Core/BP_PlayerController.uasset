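; Player controller that runs a two-element skill system, with a separate HUD skill bar for each element.
; After a short delay on BeginPlay it spawns both starting skill sets as actors into free hotkey slots.
; Swapping element toggles the visible bar, and skill keys trigger the matching skill in the active one.
; Casting disables other hotkeys on the first bar only; interact and consumable inputs just print placeholders.
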(event `self.ReceiveBeginPlay`
  (`KismetSystemLibrary.Delay` 0.2)
  (bind _asbp_hud (cast `/Game/Core/BP_HUD` (`self.GetHUD`)))
  (set `self.HUDMain` (`/Game/Core/BP_HUD.Main` _asbp_hud))
  (`self.GenerateStartingSkills_1`)
  (`self.GenerateStartingSkills_2`))

(event `InputAction|Interact`
  (params (Key :type "Key Structure" :default "AnyKey"))
  ;[1 1 1] Interact with item (that is being hovered)
  (:`Pressed`
    (`KismetSystemLibrary.PrintString` "Interact")))

(event `InputAction|UseConsumable`
  (params (Key :type "Key Structure" :default "AnyKey"))
  (bind _consumableitemslot (`self.ConsumableItemSlot`))
  ;[1 1 1] Use consumable item (from slot)
  (:`Pressed`
    (`/Engine/EditorBlueprintResources/StandardMacros.IsValid` _consumableitemslot
      (:`Is Valid`
        (if (`|EnumInequality` (`/Game/Items/BP_ConsumableItem.ConsumableType` _consumableitemslot) "NewEnumerator5")
          (`KismetSystemLibrary.PrintString` "Use Consumable"))))))

(event `InputAction|SwapElement`
  (params (Key :type "Key Structure" :default "AnyKey"))
  ;[1 1 1] Swap Element
  (:`Pressed`
    (`self.WantsToSwapElement`)))

(event `WantsToSwapElement`
  (bind _hudmain (`self.HUDMain`))
  ;[1 1 1] Swap Element
  (if (== (`self.CurrentElement`) (`self.Element_1`))
    (set `self.CurrentElement` (`self.Element_2`))
    (`Widget.SetVisibility` (`/Game/UI/WBP_Main.SkillBarContainer_1` _hudmain) "Hidden")
    (`Widget.SetVisibility` (`/Game/UI/WBP_Main.SkillBarContainer_2` _hudmain) "Visible")
    (else
      (set `self.CurrentElement` (`self.Element_1`))
      (`Widget.SetVisibility` (`/Game/UI/WBP_Main.SkillBarContainer_1` _hudmain) "Visible")
      (`Widget.SetVisibility` (`/Game/UI/WBP_Main.SkillBarContainer_2` _hudmain) "Hidden"))))

(event `WantsToUseSkill`
  (params (Hotkey :type "Key Structure" :default "AnyKey"))
  ;[1 1 1] Use Skill 1, 2, 3, 4
  (if (== (`self.CurrentElement`) (`self.Element_1`))
    (for _array_element (`/Game/UI/WBP_Main.AllHotkeySlots_1` (`self.HUDMain`))
      (bind _assignedskill (`/Game/UI/WBP_SkillHotkey.AssignedSkill` _array_element))
      (if (and (== (`/Game/UI/WBP_SkillHotkey.Hotkey` _array_element) Hotkey) (`KismetSystemLibrary.IsValid` _assignedskill))
        (`/Game/Abilities/Skills/BP_Skill.AttemptUseSkill` _assignedskill)
        (break)))
    (elif (== (`self.CurrentElement`) (`self.Element_2`))
      (for _array_element_2 (`/Game/UI/WBP_Main.AllHotkeySlots_2` (`self.HUDMain`))
        (bind _assignedskill_2 (`/Game/UI/WBP_SkillHotkey.AssignedSkill` _array_element_2))
        (if (and (== (`/Game/UI/WBP_SkillHotkey.Hotkey` _array_element_2) Hotkey) (`KismetSystemLibrary.IsValid` _assignedskill_2))
          (`/Game/Abilities/Skills/BP_Skill.AttemptUseSkill` _assignedskill_2)
          (break))))))

(event `InputAction|SkillSlot_1`
  (params (Key :type "Key Structure" :default "AnyKey"))
  ;[1 1 1] Use Skill 1, 2, 3, 4
  (:`Pressed`
    (`self.WantsToUseSkill` Key)))

(event `InputAction|SkillSlot_2`
  (params (Key :type "Key Structure" :default "AnyKey"))
  ;[1 1 1] Use Skill 1, 2, 3, 4
  (:`Pressed`
    (`self.WantsToUseSkill` Key)))

(event `InputAction|SkillSlot_3`
  (params (Key :type "Key Structure" :default "AnyKey"))
  ;[1 1 1] Use Skill 1, 2, 3, 4
  (:`Pressed`
    (`self.WantsToUseSkill` Key)))

(event `InputAction|SkillSlot_4`
  (params (Key :type "Key Structure" :default "AnyKey"))
  ;[1 1 1] Use Skill 1, 2, 3, 4
  (:`Pressed`
    (`self.WantsToUseSkill` Key)))

(fn `BeginSkillCast`
  (params (CastedSKill :type "/Game/Abilities/Skills/BP_Skill Object Reference"))
  (set `self.CurrentSkill` CastedSKill)
  (set `self.IsCasting` true)
  (for _array_element (`/Game/UI/WBP_Main.AllHotkeySlots_1` (`self.HUDMain`))
    (bind _assignedskill (`/Game/UI/WBP_SkillHotkey.AssignedSkill` _array_element))
    (`/Engine/EditorBlueprintResources/StandardMacros.IsValid` _assignedskill
      (:`Is Valid`
        (if (!= _assignedskill CastedSKill)
          (`/Game/UI/WBP_SkillHotkey.DisableHotkey` _array_element))))))

(fn `EndSpellCast`
  (params (CastedSKill :type "/Game/Abilities/Skills/BP_Skill Object Reference"))
  (set `self.CurrentSkill` null)
  (set `self.IsCasting` false)
  (for _array_element (`/Game/UI/WBP_Main.AllHotkeySlots_1` (`self.HUDMain`))
    (bind _assignedskill (`/Game/UI/WBP_SkillHotkey.AssignedSkill` _array_element))
    (`/Engine/EditorBlueprintResources/StandardMacros.IsValid` _assignedskill
      (:`Is Valid`
        (if (!= _assignedskill CastedSKill)
          (`/Game/UI/WBP_SkillHotkey.EnableHotKey` _array_element))))))

(fn `GenerateStartingSkills_1`
  (for _array_element (`self.StartingSkills_1`)
    (bind _returnvalue (`|SpawnActorFromClass` _array_element (`KismetMathLibrary.MakeTransform` (0.0 0.0 0.0)) "AlwaysSpawn" "OverrideRootScale" self))
    (for _array_element_2 (`/Game/UI/WBP_Main.AllHotkeySlots_1` (`self.HUDMain`))
      (`/Engine/EditorBlueprintResources/StandardMacros.IsValid` (`/Game/UI/WBP_SkillHotkey.AssignedSkill` _array_element_2)
        (:`Is Not Valid`
          (`/Game/UI/WBP_SkillHotkey.AssignSkill` _array_element_2 _returnvalue)
          (break))))))

(fn `GenerateStartingSkills_2`
  (for _array_element (`self.StartingSkills_2`)
    (bind _returnvalue (`|SpawnActorFromClass` _array_element (`KismetMathLibrary.MakeTransform` (0.0 0.0 0.0)) "AlwaysSpawn" "OverrideRootScale" self))
    (for _array_element_2 (`/Game/UI/WBP_Main.AllHotkeySlots_2` (`self.HUDMain`))
      (`/Engine/EditorBlueprintResources/StandardMacros.IsValid` (`/Game/UI/WBP_SkillHotkey.AssignedSkill` _array_element_2)
        (:`Is Not Valid`
          (`/Game/UI/WBP_SkillHotkey.AssignSkill` _array_element_2 _returnvalue)
          (break))))))

(fn `UserConstructionScript`)