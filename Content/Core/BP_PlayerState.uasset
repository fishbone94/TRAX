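; Player state that holds health and stamina and drives the player pawn's movement and sprinting.
; After a short delay on BeginPlay it caches player 0's BP_PlayerPawn, then forwards movement input along control-rotation yaw.
; Tick drains stamina while sprinting and regenerates it otherwise, in fixed per-frame steps without delta-time scaling.
; Sprinting starts only above a stamina threshold and falls back to walking when stamina runs out.
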(event `self.ReceiveBeginPlay`
  (`KismetSystemLibrary.Delay` 0.2)
  (bind _asbp_player_pawn (cast `/Game/Player/BP_PlayerPawn` (`GameplayStatics.GetPlayerPawn` 0)))
  (set `self.PlayerPawn` _asbp_player_pawn))

(event `self.ReceiveTick`
  (params (DeltaSeconds :type "Float (single-precision)"))
  (`|ExecutionSequence`
    (:`then_0`
      (if (`self.IsSprinting`)
        (`self.DegenStamina`)
        (else
          (`self.RegenStamina`))))))

(event `RegenStamina`
  ;[1 1 1] Regen Stamina
  (if (< (`self.Stamina`) (`self.StaminaMax`))
    (`self.ChangeStamina` 0.5)))

(event `WantsToSprint`
  ;[1 1 1] Sprint
  (if (>= (`self.Stamina`) 100.0)
    (set `self.IsSprinting` true)
    (`/Game/Player/BP_PlayerPawn.BeginSprint` (`self.PlayerPawn`))))

(event `WantsToWalk`
  ;[1 1 1] Walk
  (set `self.IsSprinting` false)
  (`/Game/Player/BP_PlayerPawn.BeginWalk` (`self.PlayerPawn`)))

(event `DegenStamina`
  ;[1 1 1] Degen Stamina
  (if (<= (`self.Stamina`) 1.0)
    (set `self.IsSprinting` false)
    (`/Game/Player/BP_PlayerPawn.BeginWalk` (`self.PlayerPawn`))
    (else
      (`self.ChangeStamina` -1.0))))

(event `MoveForward`
  (params (InputAxis :type "Float (double-precision)"))
  (bind _playerpawn (`self.PlayerPawn`))
  ;[1 1 1] Movement
  (`Pawn.AddMovementInput` _playerpawn (`KismetMathLibrary.GetForwardVector` (`KismetMathLibrary.MakeRotator` 0.0 0.0 (.yaw (`Pawn.GetControlRotation` _playerpawn)))) InputAxis false))

(event `MoveRight`
  (params (InputAxis :type "Float (double-precision)"))
  (bind _playerpawn (`self.PlayerPawn`))
  ;[1 1 1] Movement
  (`Pawn.AddMovementInput` _playerpawn (`KismetMathLibrary.GetRightVector` (`KismetMathLibrary.MakeRotator` 0.0 0.0 (.yaw (`Pawn.GetControlRotation` _playerpawn)))) InputAxis false))

(fn `ChangeHealth`
  (params (HealthInput :type "Float (double-precision)"))
  (set `self.Health` (+ HealthInput (`self.Health`))))

(fn `ChangeStamina`
  (params (StaminaInput :type "Float (double-precision)"))
  (set `self.Stamina` (+ StaminaInput (`self.Stamina`))))

(fn `UserConstructionScript`)